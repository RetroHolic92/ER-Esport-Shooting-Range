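; Shooting target that jumps to a random point in a box around BP_TargetSpawnner at start and whenever damaged.
; Each hit updates the cached player's score and hit count, then shrinks the sphere down to a size threshold, raising points per hit as it shrinks.
; It also times the interval between hits, tracking the best reaction time, and prints stats including hit rate.
; The game mode's start call sits behind an always-false check.
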(event EventBeginPlay
  (Variables|Default|SetCurrent%20Scale (Transformation|GetWorldScale (Variables|Default|GetSphere)))
  (CallFunction|TeleporttoRandomPositioninRange)
  (CallFunction|CacheGameMode)
  (CallFunction|CachePlayer))

(event Collision|EventActorBeginOverlap
  (params (OtherActor :type Actor%20Object%20Reference)))

(event EventTick
  (params (DeltaSeconds :type Float%20%28single-precision%29)))

(event Game|Damage|EventAnyDamage
  (params (Damage :type Float%20%28single-precision%29) (DamageType :type Damage%20Type%20Object%20Reference) (InstigatedBy :type Controller%20Object%20Reference) (DamageCauser :type Actor%20Object%20Reference))
  (CallFunction|UpdateScore)
  (bind _output_get (CallFunction|EndTimer))
  (Development|PrintString (Utilities|String|ToString(Float) _output_get))
  (CallFunction|UpdateReactionTime)
  (CallFunction|TeleporttoRandomPositioninRange)
  (CallFunction|ReduceObjectSize)
  (CallFunction|StartTimer))

(fn ConstructionScript)

(fn TeleporttoRandomPositioninRange
  (bind _returnvalue (Actor|GetActorOfClass "/Game/Blueprints/BP_TargetSpawnner.BP_TargetSpawnner_C"))
  (Transformation|Teleport (Math|Random|RandomPointinBoundingBox (Transformation|GetActorLocation _returnvalue) (Math|Vector|MakeVector 1e+02 2e+02 2e+02)) "0, 0, 0"))

(fn ReduceObjectSize
  (bind _sphere (Variables|Default|GetSphere))
  (bind _returnvalue (Transformation|GetWorldScale _sphere))
  (if (>= (.x _returnvalue) 0.3)
    (Transformation|SetWorldScale3D (Variables|Default|GetSphere) (Math|Vector|MakeVector (- (.x _returnvalue) (Variables|Default|GetScale%20Decrease%20when%20hit)) (- (.y _returnvalue) (Variables|Default|GetScale%20Decrease%20when%20hit)) (- (.z _returnvalue) (Variables|Default|GetScale%20Decrease%20when%20hit))))
    (Variables|Default|SetHit%20Score (+ (Variables|Default|GetHit%20Score) (Variables|Default|GetHit%20Score%20Increase)))))

(fn StartTimer
  (Variables|Default|SetSpawn%20Timestamp (Math|DateTime|Now)))

(fn EndTimer
  (bind _output_get (Variables|Default|SetReaction%20Time (Class|KismetMathLibrary|GetTotalMilliseconds (- (Math|DateTime|Now) (Variables|Default|GetSpawn%20Timestamp)))))
  (return _output_get))

(fn UpdateReactionTime
  (if (== (Variables|Default|GetBest%20Reaction%20Time) 0.0)
    (bind _output_get (Variables|Default|SetBest%20Reaction%20Time (Variables|Default|GetReaction%20Time) :!label _label))
    (Development|PrintString (Utilities|String|Append "New Best Reaction Time: " (Utilities|String|ToString(Float) _output_get)))
    (elif (< (Variables|Default|GetReaction%20Time) (Variables|Default|GetBest%20Reaction%20Time))
      (goto _label))))

(fn CacheGameMode
  (bind _asbp_shooting_game_mode (Utilities|Casting|CastToBP_ShootingGameMode (Game|GetGameMode)))
  (Variables|Default|SetAs%20BP%20Shooting%20Game%20Mode _asbp_shooting_game_mode))

(fn UpdateScore
  (bind _player (Variables|Default|GetPlayer))
  (bind _hit (Variables|/Game/FPS_Game/Blueprints/BP_CharacterBase.BP_CharacterBase_C|GetHit _player))
  (bind _shoot_count (Variables|/Game/FPS_Game/Blueprints/BP_CharacterBase.BP_CharacterBase_C|GetShoot%20Count _player))
  (bind _output_get (Variables|/Game/FPS_Game/Blueprints/BP_CharacterBase.BP_CharacterBase_C|SetScore _player (+ (Variables|/Game/FPS_Game/Blueprints/BP_CharacterBase.BP_CharacterBase_C|GetScore _player) (Variables|Default|GetHit%20Score))))
  (bind _result (Math|Float|IncrementFloat _hit)
    (:%20%20
      (if (== 0 1)
        (Default|CallGameStarts (Variables|Default|GetAs%20BP%20Shooting%20Game%20Mode)))
      (Development|PrintString (Utilities|String|Append "Score: " (Utilities|String|ToString(Integer) _output_get)))
      (Development|PrintString (Utilities|String|Append "Hit: " (Utilities|String|ToString(Float) _result)))
      (Development|PrintString (Utilities|String|Append "Shoot: " (Utilities|String|ToString(Float) _shoot_count)))
      (Development|PrintString (Utilities|String|Append "Hit Rate: " (Utilities|String|ToString(Float) (/ _hit _shoot_count)))))))

(fn CachePlayer
  (bind _returnvalue (Actor|GetActorOfClass "/Game/FPS_Game/Blueprints/BP_CharacterBase.BP_CharacterBase_C"))
  (Variables|Default|SetPlayer _returnvalue))